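; BP_HitSplat is an actor that displays a damage number as a hit splat.
; On BeginPlay it passes DamageAmount to either the HitSplat or HitSplatMissed widget, using the missed one for zero damage, and hides the other.
; It then stores its location and starts a countdown.
; Tick decrements the countdown, which nothing here reads, and sweeps the actor to the unchanged stored location.
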(event EventBeginPlay
  (if (== (Variables|Default|Getdamage%20Amount) 0.0)
    (bind _ashit_splat_missed (Utilities|Casting|CastToHitSplatMissed (UserInterface|GetWidget (Variables|Default|GetWidgetMissed))))
    (Variables|/Game/GUI/HitSplatMissed.HitSplatMissed_C|SetdamageAmount _ashit_splat_missed (Variables|Default|Getdamage%20Amount))
    (Widget|SetVisibility (UserInterface|GetWidget (Variables|Default|GetWidget)) "Hidden")
    (else
      (bind _ashit_splat (Utilities|Casting|CastToHitSplat (UserInterface|GetWidget (Variables|Default|GetWidget))))
      (Variables|/Game/GUI/HitSplat.HitSplat_C|SetdamageAmount _ashit_splat (Variables|Default|Getdamage%20Amount))
      (Widget|SetVisibility (UserInterface|GetWidget (Variables|Default|GetWidgetMissed)) "Hidden")))
  (Variables|Default|SetcurrentLocation (Transformation|GetActorLocation))
  (Variables|Default|SettimeRemaining 1.5))

(event EventTick
  (params (DeltaSeconds :type Float%20%28single-precision%29))
  (Variables|Default|SetDelta%20Seconds DeltaSeconds)
  (Variables|Default|SettimeRemaining (- (Variables|Default|GettimeRemaining) (Variables|Default|GetDelta%20Seconds)))
  (Transformation|SetActorLocation (Variables|Default|GetcurrentLocation) true false))

(fn ConstructionScript)