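; BP_Item is a pickup actor that reports its item to the caller's inventory when picked up.
; PickUpItem acts only while its BPCClickableComponent is hovered, and refuses with an "Inventory full" message once the passed-in counter reaches the slot limit.
; Otherwise it increments the counter, returns the item with a success flag, and calls DestroyItem, which removes the actor after a short delay.
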(event Custom|Destroy%20Item
  (Utilities|FlowControl|Delay 0.1)
  (Actor|DestroyActor))

(event EventBeginPlay)

(event Collision|EventActorBeginOverlap
  (params (OtherActor :type Actor%20Object%20Reference)))

(event EventTick
  (params (DeltaSeconds :type Float%20%28single-precision%29)))

(fn ConstructionScript)

(fn PickUpItem
  (params (Counter :type Integer))
  (if (Variables|/Game/Inventory/BPC_ClickableComponent.BPC_ClickableComponent_C|GetIsHovered (Variables|Default|GetBPC_ClickableComponent))
    (if (>= Counter 8)
      (Development|PrintString "Inventory full")
      (else
        (Development|PrintString "Item picked")
        (Math|Integer|IncrementInt Counter
          (:%20%20
            (CallFunction|DestroyItem)
            (return (Variables|Default|GetItem) true Counter))))))
  (return "" false Counter))