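; BPC_ClickableComponent is an actor component that makes its owner respond to mouse hover and clicks.
; On BeginPlay it binds the owner's click event and, if a static mesh component exists, its cursor-over events.
; Hovering toggles custom depth on that mesh, typically for outline highlighting, and tracks IsHovered.
; The click handler is empty; a click-toggle material swap remains as unconnected, never-run logic.
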(event Custom|OnMouseClicked
  (params (TouchedActor :type Actor%20Object%20Reference) (ButtonPressed :type Key%20Structure :default "None")))

(event Custom|OnMouseOver
  (params (TouchedActor :type Actor%20Object%20Reference))
  (Rendering|SetRenderCustomDepth (Variables|Default|GetStaticMeshRef) true)
  (Variables|Default|SetIsHovered true))

(event Custom|OnMouseHoverEnd
  (params (TouchedActor :type Actor%20Object%20Reference))
  (Rendering|SetRenderCustomDepth (Variables|Default|GetStaticMeshRef) false)
  (Variables|Default|SetIsHovered false))

(event EventBeginPlay
  (bind _returnvalue (Components|GetOwner))
  (bind _returnvalue_2 (Actor|GetComponentbyClass _returnvalue "/Script/Engine.StaticMeshComponent"))
  (EventDispatchers|BindEventtoOnClicked _returnvalue (delegate Custom|OnMouseClicked))
  (Utilities|IsValid _returnvalue_2
    (:Is%20Valid
      (Variables|Default|SetStaticMeshRef _returnvalue_2)
      (EventDispatchers|BindEventtoOnBeginCursorOver _returnvalue (delegate Custom|OnMouseOver))
      (EventDispatchers|BindEventtoOnEndCursorOver _returnvalue (delegate Custom|OnMouseHoverEnd)))))